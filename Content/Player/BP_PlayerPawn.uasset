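; Player pawn that aims its weapon with the camera and fires projectiles on left mouse click.
; Tick matches the mesh's world rotation to the player camera's rotation.
; Firing spawns BP_Projectile at the Muzzle and broadcasts a PlayerFire gameplay tag event through GameplayActionSubsystem, with the pawn as instigator and projectile as trigger.
; A timeline recoil curve then animates the weapon arrow's relative X location.
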(event `self.ReceiveTick`
  (params (DeltaSeconds :type "Float (single-precision)"))
  (bind _returnvalue (`GameplayStatics.GetPlayerCameraManager` 0))
  ;[1 1 1] update weapon arrow  rotation
  (`/Engine/EditorBlueprintResources/StandardMacros.IsValid` _returnvalue
    (:`Is Valid`
      (`SceneComponent.K2_SetWorldRotation` (`self.MeshComponent`) (`PlayerCameraManager.GetCameraRotation` _returnvalue) false false))))

(event `Key|LeftMouseButton`
  (params (Key :type "Key Structure"))
  (bind _weaponarrow (`self.WeaponArrow`))
  (bind (_relativelocation_x _relativelocation_y _relativelocation_z) (`KismetMathLibrary.BreakVector` (`SceneComponent.RelativeLocation` _weaponarrow)))
  (:`Pressed`
    ;[1 1 1] fire
    (bind _returnvalue (`|SpawnActorFromClass` "/Game/Projectiles/BP_Projectile.BP_Projectile_C" (`SceneComponent.K2_GetComponentToWorld` (`self.Muzzle`)) "Undefined" "OverrideRootScale" self self))
    ;[1 1 1] trigger action event
    (`GameplayActionSubsystem.BroadcastGameplayActionEvent` (subsystem `GameplayActionSubsystem`) (`BlueprintGameplayTagLibrary.MakeLiteralGameplayTag` (struct :`TagName` "GameplayActionEvent.PlayerFire")) self _returnvalue)
    ;[1 1 1] weapon fire animation
    (bind (_direction _recoilcurve) (`Timeline|WeaponFireAnimTimeline` :!via `PlayFromStart`)
      (:`Update`
        (`SceneComponent.K2_SetRelativeLocation` _weaponarrow (`KismetMathLibrary.MakeVector` _recoilcurve _relativelocation_y _relativelocation_z) false false)))))

(fn `UserConstructionScript`)
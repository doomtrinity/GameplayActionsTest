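; Cheat manager Blueprint for debugging Blueprint-bindable gameplay action delegates.
; Paired add and remove events bind or unbind handlers for action started, stopped and event-triggered delegates on the first gameplay action component found.
; The handlers print the owner and action tag, plus the aborted flag for stops or the event tag, instigator and trigger for triggered events.
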(event `self.GameplayActions_AddActionStartedDynamicDelegate`
  ;[1 1 1] debug blueprint action started events
  (message `GameplayActionInterface.AddActionStartedDynamicDelegate` (`self.FindFirstGameplayActionComponent`) (delegate `ActionStartedEvent`)))

(event `ActionStartedEvent`
  (params (InActionOwner :type "Actor Object Reference") (InActionTag :type "GameplayTag Structure (by ref)"))
  ;[1 1 1] debug blueprint action started events
  (`KismetSystemLibrary.PrintString` (`KismetStringLibrary.Concat_StrStr` (`KismetSystemLibrary.GetObjectName` InActionOwner) " handling action started: " (`KismetStringLibrary.Conv_NameToString` (`BlueprintGameplayTagLibrary.GetTagName` InActionTag)))))

(event `self.GameplayActions_RemoveActionStartedDynamicDelegate`
  ;[1 1 1] debug blueprint action started events
  (message `GameplayActionInterface.RemoveActionStartedDynamicDelegate` (`self.FindFirstGameplayActionComponent`) (delegate `ActionStartedEvent`)))

(event `self.GameplayActions_AddActionStoppedDynamicDelegate`
  ;[1 1 1] debug action stopped blueprint events
  (message `GameplayActionInterface.AddActionStoppedDynamicDelegate` (`self.FindFirstGameplayActionComponent`) (delegate `ActionStoppedEvent`)))

(event `ActionStoppedEvent`
  (params (InActionOwner :type "Actor Object Reference") (InActionTag :type "GameplayTag Structure (by ref)") (bInActionAborted :type Boolean))
  ;[1 1 1] debug action stopped blueprint events
  (`KismetSystemLibrary.PrintString` (`KismetStringLibrary.Concat_StrStr` (`KismetSystemLibrary.GetObjectName` InActionOwner) " handling action stopped: " (`KismetStringLibrary.Conv_NameToString` (`BlueprintGameplayTagLibrary.GetTagName` InActionTag)) " aborted: " (`KismetStringLibrary.Conv_BoolToString` bInActionAborted))))

(event `self.GameplayActions_RemoveActionStoppedDynamicDelegate`
  ;[1 1 1] debug action stopped blueprint events
  (message `GameplayActionInterface.RemoveActionStoppedDynamicDelegate` (`self.FindFirstGameplayActionComponent`) (delegate `ActionStoppedEvent`)))

(event `self.GameplayActions_AddActionEventDynamicDelegate`
  ;[1 1 1] debug action event triggered blueprint events
  (message `GameplayActionInterface.AddActionEventDynamicDelegate` (`self.FindFirstGameplayActionComponent`) (delegate `ActionEventTriggeredEvent`)))

(event `ActionEventTriggeredEvent`
  (params (InActionOwner :type "Actor Object Reference") (InActionTag :type "GameplayTag Structure (by ref)") (InEventTag :type "GameplayTag Structure (by ref)") (InInstigator :type "Actor Object Reference") (InTrigger :type "Actor Object Reference"))
  ;[1 1 1] debug action event triggered blueprint events
  (`KismetSystemLibrary.PrintString` (`KismetStringLibrary.Concat_StrStr` "action owner: " (`KismetSystemLibrary.GetObjectName` InActionOwner) ", action tag: " (`KismetStringLibrary.Conv_NameToString` (`BlueprintGameplayTagLibrary.GetTagName` InActionTag)) ", event tag: " (`KismetStringLibrary.Conv_NameToString` (`BlueprintGameplayTagLibrary.GetTagName` InEventTag)) ", instigator: " (`KismetSystemLibrary.GetObjectName` InInstigator) ", trigger: " (`KismetSystemLibrary.GetObjectName` InTrigger))))

(event `self.GameplayActions_RemoveActionEventDynamicDelegate`
  ;[1 1 1] debug action event triggered blueprint events
  (message `GameplayActionInterface.RemoveActionEventDynamicDelegate` (`self.FindFirstGameplayActionComponent`) (delegate `ActionEventTriggeredEvent`)))
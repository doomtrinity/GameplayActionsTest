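; BP_AI_Controller is an AI controller that initializes brain logic for possessed pawns and caches their target actor.
; On possession it sets up Blackboard_AI and, if that succeeds, starts its BehaviorTree component's logic.
; A BP_AI_Character can opt out via StartBrainLogicOnPossess, while any other pawn type always starts.
; UpdateTargetActorCache stores the target, which GetTargetActor returns without a blackboard lookup.
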(event `self.ReceivePossess`
  (params (PossessedPawn :type "Pawn Object Reference"))
  (bind _asbp_ai_character (cast `/Game/AI/BP_AI_Character` PossessedPawn)
    (:`then`
      (if (`/Game/AI/BP_AI_Character.bStartBrainLogicOnPossess` _asbp_ai_character)
        (bind (_blackboardcomponent _returnvalue) (`self.UseBlackboard` "/Game/AI/BehaviorTrees/Blackboard_AI.Blackboard_AI" :!label _label))
        (if _returnvalue
          (`BrainComponent.StartLogic` (`self.BehaviorTree`)))))
    (:`CastFailed`
      (goto _label))))

(event `UpdateTargetActorCache`
  (params (TargetActor :type "Actor Object Reference"))
  (set `self.TargetActorCache` TargetActor))

(fn `GetTargetActor`
  (returns (TargetActor :type "Actor Object Reference"))
  (return (`self.TargetActorCache`)))

(fn `UserConstructionScript`)
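; AI character Blueprint that handles health, stagger, death and simple attacks through a gameplay action component.
; Damage lowers health and fills a decaying accumulator, triggering Stagger past a threshold or Death at zero health.
; Timelines fake melee animation by moving the mesh and flash its color on hits, while stagger sets its own color.
; It also fires projectiles from a muzzle, and OnDeath swaps the hidden actor for an impulse-launched ragdoll.
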(event `self.ReceiveBeginPlay`
  (bind _gameplayactioncomp (`self.GameplayActionComp`))
  ;[1 1 1] init
  (set `self.CurrentHealth` (`self.StartingHealth`))
  (set `self.AccumulatedDamage` 0.0)
  (`GameplayActionInterface.AddActionStoppedDynamicDelegate` _gameplayactioncomp (delegate `HandleActionStopped`))
  (`GameplayActionInterface.AddActionStartedDynamicDelegate` _gameplayactioncomp (delegate `HandleActionStarted`))
  (set `self.CachedMeshInitialTransform` (`SceneComponent.GetRelativeTransform` (`self.PawnMesh`))))

(event `HandleActionStarted`
  (params (InActionOwner :type "Actor Object Reference") (InActionTag :type "GameplayTag Structure (by ref)"))
  ;[1 1 1] handle action started and stopped
  (if (== InActionTag (struct :`TagName` "GameplayAction.Stagger"))
    (`self.HandleStaggerStarted`)))

(event `HandleActionStopped`
  (params (InActionOwner :type "Actor Object Reference") (InActionTag :type "GameplayTag Structure (by ref)") (bInActionAborted :type Boolean))
  ;[1 1 1] handle action started and stopped
  (if (== InActionTag (struct :`TagName` "GameplayAction.Stagger"))
    (`self.HandleStaggerStopped`)))

(event `self.ReceiveTick`
  (params (DeltaSeconds :type "Float (single-precision)"))
  (bind _accumulateddamage (`self.AccumulatedDamage`))
  ;[1 1 1] tick
  ;[1 1 1] accumulated damage logic
  (if (> _accumulateddamage 0.0)
    (bind _output_get (set `self.AccumulatedDamage` (- _accumulateddamage (* (`GameplayStatics.GetWorldDeltaSeconds`) (`self.AccumulatedDamageDecreaseRate`))))))
  ;[1 1 1] print debug data
  (`KismetSystemLibrary.PrintString` (`KismetStringLibrary.Concat_StrStr` "accumulated damage: " (`KismetStringLibrary.Conv_DoubleToString` _output_get) " health: " (`KismetStringLibrary.Conv_IntToString` (`self.CurrentHealth`))) false false (struct :`G` 0.66 :`B` 1.0 :`A` 1.0) 0.0))

(event `StopMeleeAnim`
  (bind _pawnmesh (`self.PawnMesh`))
  ;[1 1 1] melee anim
  (`TimelineComponent.Stop` (`self.MeleeAnimTimeline`))
  (`SceneComponent.K2_SetRelativeRotation` _pawnmesh (.rotation (`self.CachedMeshInitialTransform`)) false false :!label _label)
  (`SceneComponent.K2_SetRelativeLocation` _pawnmesh (.location (`self.CachedMeshInitialTransform`)) false false))

(event `PlayMeleeAnim`
  (params (AnimSpeed :type "Float (double-precision)" :default 1.0))
  (bind _pawnmesh (`self.PawnMesh`))
  ;[1 1 1] melee anim
  (`TimelineComponent.SetPlayRate` (`self.MeleeAnimTimeline`) AnimSpeed)
  (bind (_direction _meleeposition _meleerotation) (`Timeline|MeleeAnimTimeline` :`NewTime` 1.0 :!via `PlayFromStart`)
    (:`Update`
      (`SceneComponent.K2_SetRelativeRotation` _pawnmesh (`KismetMathLibrary.MakeRotator` (.roll (.rotation (`self.CachedMeshInitialTransform`))) _meleerotation (.yaw (.rotation (`self.CachedMeshInitialTransform`)))) false false)
      (`SceneComponent.K2_SetRelativeLocation` _pawnmesh (`KismetMathLibrary.MakeVector` _meleeposition (.y (.location (`self.CachedMeshInitialTransform`))) (.z (.location (`self.CachedMeshInitialTransform`)))) false false))
    (:`Finished`
      (`self.OnMeleeAnimEnd`)
      (goto _label))))

(event `self.ReceiveAnyDamage`
  (params (Damage :type "Float (single-precision)") (DamageType :type "DamageType Object Reference") (InstigatedBy :type "Controller Object Reference") (DamageCauser :type "Actor Object Reference"))
  ;[1 1 1] handle damage
  (`KismetSystemLibrary.PrintString` (`KismetStringLibrary.Concat_StrStr` "on take damage, causer: " (`KismetSystemLibrary.GetObjectName` DamageCauser) " instigator: " (`KismetSystemLibrary.GetObjectName` InstigatedBy) " damage: " (`KismetStringLibrary.Conv_DoubleToString` Damage)) false)
  (set `self.AccumulatedDamage` (+ Damage (`self.AccumulatedDamage`)))
  (bind _output_get (set `self.CurrentHealth` (- (`self.CurrentHealth`) (`KismetMathLibrary.FTrunc` Damage))))
  (if (> _output_get 0)
    (`self.TryStartStagger` InstigatedBy DamageCauser)
    ;[1 1 1] change mesh color on damage
    (if (not (`GameplayActionInterface.IsActionActive` (`self.GameplayActionComp`) (`BlueprintGameplayTagLibrary.MakeLiteralGameplayTag` (struct :`TagName` "GameplayAction.Stagger"))))
      (bind (_direction _damagecolor) (`Timeline|DamageTimeline` :!via `PlayFromStart`)
        (:`Update`
          (`MeshComponent.SetVectorParameterValueOnMaterials` (`self.PawnMesh`) "Color" (`KismetMathLibrary.Conv_LinearColorToVector` _damagecolor)))))
    (else
      (`GameplayActionInterface.TriggerActionEvent` (`self.GameplayActionComp`) (`BlueprintGameplayTagLibrary.MakeLiteralGameplayTag` (struct :`TagName` "GameplayActionEvent.Death")) InstigatedBy DamageCauser))))

(event `ResetAccumulatedDamage`
  ;[1 1 1] handle damage
  (set `self.AccumulatedDamage` 0.0))

(event `TryStartStagger`
  (params (Instigator :type "Controller Object Reference") (DamageCauser :type "Actor Object Reference"))
  ;[1 1 1] stagger events
  (if (`GameplayActionInterface.IsActionActive` (`self.GameplayActionComp`) (`BlueprintGameplayTagLibrary.MakeLiteralGameplayTag` (struct :`TagName` "GameplayAction.Stagger")))
    _
    (elif (> (`self.AccumulatedDamage`) (`self.StaggerDamage`))
      (`GameplayActionInterface.TriggerActionEvent` (`self.GameplayActionComp`) (`BlueprintGameplayTagLibrary.MakeLiteralGameplayTag` (struct :`TagName` "GameplayActionEvent.Stagger")) Instigator DamageCauser))))

(event `HandleStaggerStarted`
  ;[1 1 1] stagger events
  (`TimelineComponent.Stop` (`self.DamageTimeline`))
  (`MeshComponent.SetVectorParameterValueOnMaterials` (`self.PawnMesh`) "Color" (`KismetMathLibrary.Conv_LinearColorToVector` (`self.StaggerMeshColor`))))

(event `HandleStaggerStopped`
  ;[1 1 1] stagger events
  (`self.ResetAccumulatedDamage`)
  (`MeshComponent.SetVectorParameterValueOnMaterials` (`self.PawnMesh`) "Color" (`KismetMathLibrary.Conv_LinearColorToVector` (`self.DefaultMeshColor`))))

(event `FireProjectile`
  ;[1 1 1] fire projectile
  (`|SpawnActorFromClass` "/Game/Projectiles/BP_Projectile.BP_Projectile_C" (`SceneComponent.K2_GetComponentToWorld` (`self.Muzzle`)) "Undefined" "OverrideRootScale" self self))

(event `OnDeath`
  ;[1 1 1] handle death
  (`self.SetActorEnableCollision` false)
  (`MovementComponent.StopMovementImmediately` (`self.CharacterMovement`))
  (`self.SetActorHiddenInGame` true)
  (bind _returnvalue (`|SpawnActorFromClass` "/Game/AI/BP_Ragdoll.BP_Ragdoll_C" (`self.GetTransform`) "Undefined" "OverrideRootScale" null null))
  (if (`KismetSystemLibrary.IsValid` _returnvalue)
    (`PrimitiveComponent.AddImpulse` (`StaticMeshActor.StaticMeshComponent` _returnvalue) (* (`KismetMathLibrary.Normal` (* (`self.GetActorForwardVector`) -1) 0.0) 600.0) "None" true))
  (`self.SetLifeSpan` 1.0))

(fn `GetGameplayActionComponent`
  (returns (ReturnValue :type "ActorComponent Object Reference"))
  (return (`self.GameplayActionComp`)))

(fn `UserConstructionScript`)
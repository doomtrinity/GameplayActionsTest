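; Projectile actor that deals its base damage to whatever it overlaps, using a projectile damage type.
; It skips damage when the target has the same class as its instigator, a crude friendly-fire check.
; Any overlap or the movement component stopping hides the mesh and ignores all collision channels, leaving the actor alive rather than destroying it.
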(event `self.ReceiveActorBeginOverlap`
  (params (OtherActor :type "Actor Object Reference"))
  (`KismetSystemLibrary.PrintString` (`KismetStringLibrary.Concat_StrStr` "begin overlap with:  " (`KismetSystemLibrary.GetDisplayName` OtherActor)) false false)
  (if (not (== (`GameplayStatics.GetObjectClass` OtherActor) (`GameplayStatics.GetObjectClass` (`self.Instigator`))))
    (`GameplayStatics.ApplyDamage` OtherActor (`self.BaseDamage`) (`self.GetInstigatorController`) self "/Game/Projectiles/BP_DamageType_Projectile.BP_DamageType_Projectile_C"))
  (`self.StopProjectileLogic`))

(event `self.ProjectileMovement.OnProjectileStop`
  (params (ImpactResult :type "HitResult Structure (by ref)"))
  (`self.StopProjectileLogic`))

(event `StopProjectileLogic`
  (bind _staticmeshcomponent (`self.StaticMeshComponent`))
  (`SceneComponent.SetVisibility` _staticmeshcomponent false true)
  (`PrimitiveComponent.SetCollisionResponseToAllChannels` _staticmeshcomponent "ECR_Ignore"))

(fn `UserConstructionScript`)
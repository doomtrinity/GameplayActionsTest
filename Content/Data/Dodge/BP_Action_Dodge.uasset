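; Gameplay action that makes its owning pawn sidestep projectiles fired by the player.
; On a PlayerFire event, if the projectile is in front of the owner, it picks a random left or right direction, line-traces it for obstacles, tries the opposite if blocked, and sets CanDodge.
; While active, it raises walk speed to the dodge velocity and feeds movement input each tick.
; A timer stops the action, restoring speed and clearing the dodge state.
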(event `self.OnInitAction`
  ;[1 1 1] cache data
  (bind _aspawn (cast `Pawn` (`self.OwnerActor`)))
  (set `self.OwnerPawn` _aspawn)
  (bind _asdodge_action_parameters (cast `/Game/Data/Dodge/DodgeActionParameters` (`self.ActionParameters`)))
  (set `self.DodgeActionParameters` _asdodge_action_parameters)
  (bind _ascharacter_movement_component (cast `CharacterMovementComponent` (`Pawn.GetMovementComponent` (`self.OwnerPawn`))))
  (bind _output_get (set `self.MovementComp` _ascharacter_movement_component))
  (set `self.DefaultMaxWalkSpeed` (`CharacterMovementComponent.MaxWalkSpeed` _output_get)))

(event `self.OnActionEvent`
  (params (InEventTag :type "GameplayTag Structure (by ref)") (InInstigator :type "Actor Object Reference") (InTrigger :type "Actor Object Reference"))
  (bind _lastplayerprojectile (`self.LastPlayerProjectile`))
  (bind _returnvalue (`Actor.GetActorRightVector` (`self.OwnerActor`)))
  ;[1 1 1] check event tag
  (if (== InEventTag (struct :`TagName` "GameplayActionEvent.PlayerFire"))
    (set `self.LastPlayerProjectile` InTrigger)
    ;[1 1 1] determine dodge direction
    (bind _ascharacter (cast `Character` (`self.OwnerActor`)))
    (`/Engine/EditorBlueprintResources/StandardMacros.IsValid` _lastplayerprojectile
      (:`Is Valid`
        (if (> (`KismetMathLibrary.Dot_VectorVector` (`KismetMathLibrary.Normal` (- (`Actor.K2_GetActorLocation` _lastplayerprojectile) (`Actor.K2_GetActorLocation` _ascharacter))) (`Actor.GetActorForwardVector` _ascharacter)) 0.75)
          (bind _output_get (set `self.DodgeDirection` (`KismetMathLibrary.SelectVector` _returnvalue (* _returnvalue -1) (`KismetMathLibrary.RandomBool`))))
          (bind _bvaliddodgedirection (`self.ValidateDodgeDirection` _output_get))
          (if _bvaliddodgedirection
            (set `self.bCanDodge` true)
            (else
              (bind _output_get_2 (set `self.DodgeDirection` (* (`self.DodgeDirection`) -1)))
              (bind _bvaliddodgedirection_2 (`self.ValidateDodgeDirection` _output_get_2))
              (set `self.bCanDodge` _bvaliddodgedirection_2))))))))

(event `self.OnActionStarted`
  ;[1 1 1] set dodge walk speed
  (set `CharacterMovementComponent.MaxWalkSpeed` (`/Game/Data/Dodge/DodgeActionParameters.DodgeVelocity` (`self.DodgeActionParameters`)) (`self.MovementComp`))
  ;[1 1 1] set dodge timer
  (bind _returnvalue (`KismetSystemLibrary.K2_SetTimerDelegate` (delegate `OnDodgeEnd`) (`/Game/Data/Dodge/DodgeActionParameters.DodgeTimeout` (`self.DodgeActionParameters`))))
  (set `self.DodgeTimerHandle` _returnvalue))

(event `OnDodgeEnd`
  ;[1 1 1] set dodge timer
  (bind _returnvalue (message `GameplayActionOwnerInterface.GetGameplayActionComponent` (`self.OwnerActor`)))
  (message `GameplayActionInterface.StopAction` _returnvalue (`self.ActionTag`) true))

(event `self.OnActionStopped`
  (params (bInActionAborted :type Boolean))
  ;[1 1 1] reset
  (set `self.DodgeDirection` (0.0 0.0 0.0))
  (`KismetSystemLibrary.K2_ClearAndInvalidateTimerHandle` (`self.OwnerActor`) (`self.DodgeTimerHandle`))
  (set `CharacterMovementComponent.MaxWalkSpeed` (`self.DefaultMaxWalkSpeed`) (`self.MovementComp`))
  (set `self.bCanDodge` false))

(event `self.TickAction`
  (params (DeltaTime :type "Float (single-precision)"))
  ;[1 1 1] dodge movement
  (`Pawn.AddMovementInput` (`self.OwnerPawn`) (* (`self.DodgeDirection`) (* DeltaTime (`/Game/Data/Dodge/DodgeActionParameters.DodgeVelocity` (`self.DodgeActionParameters`)))) 1.0 false))

(fn `ValidateDodgeDirection`
  (params (InDodgeDirection :type "Vector Structure"))
  (returns (bValidDodgeDirection :type Boolean))
  (bind _owneractor (`self.OwnerActor`))
  (bind _returnvalue (`Actor.K2_GetActorLocation` _owneractor))
  (bind (_outhit _returnvalue_2) (`KismetSystemLibrary.LineTraceSingle` _owneractor _returnvalue (+ _returnvalue (* InDodgeDirection 180.0)) "TraceTypeQuery1" false (`|MakeArray` _owneractor)))
  (return (not _returnvalue_2)))
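; Gameplay action that runs a melee attack on an AI character owner by driving its melee animation.
; On init it caches the BP_AI_Character and MeleeActionParameters and binds to the character's melee anim end event.
; Starting plays the animation at the configured speed, and its end stops the still-active action as completed through the GameplayActionComponent.
; An aborted stop cuts the animation short.
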(event `self.OnInitAction`
  (`KismetSystemLibrary.PrintString` (`self.OwnerActor`) "melee init action" false false)
  (bind _asbp_ai_character (cast `/Game/AI/BP_AI_Character` (`self.OwnerActor`)))
  (bind _output_get (set `self.OwnerCharacter` _asbp_ai_character))
  (add `/Game/AI/BP_AI_Character.OnMeleeAnimEnd` _output_get (delegate `OnAnimEnd`))
  (bind _asmelee_action_parameters (cast `/Game/Data/Melee/MeleeActionParameters` (`self.ActionParameters`)))
  (set `self.MeleeActionParams` _asmelee_action_parameters))

(event `OnAnimEnd`
  (bind _returnvalue (message `GameplayActionOwnerInterface.GetGameplayActionComponent` (`self.OwnerActor`)))
  (bind _returnvalue_2 (message `GameplayActionInterface.IsActionActive` _returnvalue (`self.ActionTag`)))
  (if _returnvalue_2
    (message `GameplayActionInterface.StopAction` _returnvalue (`self.ActionTag`) true)))

(event `self.OnActionStarted`
  (`KismetSystemLibrary.PrintString` (`self.OwnerActor`) "melee action started" false false)
  (`/Game/AI/BP_AI_Character.PlayMeleeAnim` (`self.OwnerCharacter`) (`/Game/Data/Melee/MeleeActionParameters.MeleeAnimSpeed` (`self.MeleeActionParams`))))

(event `self.OnActionStopped`
  (params (bInActionAborted :type Boolean))
  (`KismetSystemLibrary.PrintString` (`self.OwnerActor`) "melee action stopped" false false)
  (if bInActionAborted
    (`/Game/AI/BP_AI_Character.StopMeleeAnim` (`self.OwnerCharacter`))))
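; AI gameplay action that makes an enemy strafe sideways around its target while firing projectiles on a looping timer.
; Duration and shot interval come from the strafe action parameters, and direction is randomized on each start.
; Each tick it faces the target and moves perpendicular to it, approximating an orbit without holding an exact radius.
; It stops as completed when time runs out or a sideways line trace detects an obstacle.
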(event `self.OnInitAction`
  (bind _asbp_ai_character (cast `/Game/AI/BP_AI_Character` (`self.OwnerActor`)))
  (set `self.OwnerCharacter` _asbp_ai_character)
  (bind _asbp_ai_controller (cast `/Game/AI/BP_AI_Controller` (`AIBlueprintHelperLibrary.GetAIController` (`self.OwnerActor`))))
  (set `self.OwnerController` _asbp_ai_controller)
  (bind _asstrafe_action_parameters (cast `/Game/Data/Strafe/StrafeActionParameters` (`self.ActionParameters`)))
  (bind _output_get (set `self.StrafeActionParameters` _asstrafe_action_parameters))
  (set `self.StrafeDuration` (`/Game/Data/Strafe/StrafeActionParameters.StrafeTimeDuration` _output_get))
  (set `self.TimeBetweenShots` (`/Game/Data/Strafe/StrafeActionParameters.TimeBetweenShots` _output_get)))

(event `self.OnActionStarted`
  (bind _returnvalue (`KismetSystemLibrary.K2_SetTimerDelegate` (delegate `FireProjectile`) (`self.TimeBetweenShots`) true))
  (set `self.FireProjectileTimerHandle` _returnvalue)
  (set `self.StrafeCurrentTime` 0.0)
  (set `self.bClockwiseStrafe` (`KismetMathLibrary.RandomBool`)))

(event `FireProjectile`
  (`/Game/AI/BP_AI_Character.FireProjectile` (`self.OwnerCharacter`)))

(event `self.OnActionStopped`
  (params (bInActionAborted :type Boolean))
  (`KismetSystemLibrary.K2_ClearAndInvalidateTimerHandle` (`self.OwnerActor`) (`self.FireProjectileTimerHandle`)))

(event `self.TickAction`
  (params (DeltaTime :type "Float (single-precision)"))
  (bind _ownercharacter (`self.OwnerCharacter`))
  (set `self.CachedDeltaTime` DeltaTime)
  (bind _output_get (set `self.StrafeCurrentTime` (+ (`self.StrafeCurrentTime`) (`self.CachedDeltaTime`))))
  (if (> _output_get (`self.StrafeDuration`))
    (bind _returnvalue (message `GameplayActionOwnerInterface.GetGameplayActionComponent` (`self.OwnerActor`) :!label _label))
    (message `GameplayActionInterface.StopAction` _returnvalue (`self.ActionTag`) true)
    (elif (`self.ShouldStopStrafe`)
      (goto _label)
      (else
        (`Pawn.AddMovementInput` _ownercharacter (`self.DetermineOwnerDirection`) 1.0 false)
        (`Actor.K2_SetActorRotation` _ownercharacter (`self.DetermineOwnerRotation`) false)))))

(fn `DetermineOwnerDirection`
  (returns (MovementInputVector :type "Vector Structure"))
  (return (`KismetMathLibrary.GreaterGreater_VectorRotator` (`KismetMathLibrary.SelectVector` (`KismetMathLibrary.Vector_Left`) (`KismetMathLibrary.Vector_Right`) (`self.bClockwiseStrafe`)) (`KismetMathLibrary.FindLookAtRotation` (`Actor.K2_GetActorLocation` (`self.OwnerActor`)) (`Actor.K2_GetActorLocation` (`/Game/AI/BP_AI_Controller.GetTargetActor` (`self.OwnerController`)))))))

(fn `DetermineOwnerRotation`
  (returns (Rotation :type "Rotator Structure"))
  (return (`KismetMathLibrary.FindLookAtRotation` (`Actor.K2_GetActorLocation` (`self.OwnerActor`)) (`Actor.K2_GetActorLocation` (`/Game/AI/BP_AI_Controller.GetTargetActor` (`self.OwnerController`))))))

(fn `ShouldStopStrafe`
  (returns (bStopStrafe :type Boolean))
  (bind _owneractor (`self.OwnerActor`))
  (bind _returnvalue (`Actor.K2_GetActorLocation` _owneractor))
  (bind _returnvalue_2 (`Actor.GetActorRightVector` _owneractor))
  ;[1 1 1] simple euristic check to determine if something is preventing the actor from moving i.e. there is an obstacle
  (bind (_outhit _returnvalue_3) (`KismetSystemLibrary.LineTraceSingle` (`self.OwnerActor`) _returnvalue (+ _returnvalue (* (`KismetMathLibrary.SelectVector` (* _returnvalue_2 -1.0) _returnvalue_2 (`self.bClockwiseStrafe`)) 240.0)) "TraceTypeQuery1"))
  (return _returnvalue_3))
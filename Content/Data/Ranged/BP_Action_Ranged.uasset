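; Gameplay action that makes an AI character fire projectiles repeatedly for a set duration.
; On init it reads the attack duration from RangedActionParameters, and on start a timer later stops the action as completed through the owner's gameplay action component.
; A self-rescheduling timer calls FireProjectile on the character, asking the parameters for each next delay.
; Stopping the action clears both timers.
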(event `self.OnInitAction`
  (bind _asbp_ai_character (cast `/Game/AI/BP_AI_Character` (`self.OwnerActor`)))
  (set `self.OwnerCharacter` _asbp_ai_character)
  (bind _asranged_action_parameters (cast `/Game/Data/Ranged/RangedActionParameters` (`self.ActionParameters`)))
  (bind _output_get (set `self.RangedActionParameters` _asranged_action_parameters))
  (set `self.RangedAttackTimeDuration` (`/Game/Data/Ranged/RangedActionParameters.RangedAttackTimeDuration` _output_get)))

(event `self.OnActionStarted`
  (bind _returnvalue (`KismetSystemLibrary.K2_SetTimerDelegate` (delegate `StopRangedAction`) (`self.RangedAttackTimeDuration`)))
  (set `self.RangedActionTimerHandle` _returnvalue)
  (`self.OnNextFire`))

(event `StopRangedAction`
  (bind _returnvalue (message `GameplayActionOwnerInterface.GetGameplayActionComponent` (`self.OwnerActor`)))
  (message `GameplayActionInterface.StopAction` _returnvalue (`self.ActionTag`) true))

(event `OnNextFire`
  (bind _returnvalue (`KismetSystemLibrary.K2_SetTimerDelegate` (delegate `FireProjectile`) (`/Game/Data/Ranged/RangedActionParameters.GetNextFireDelay` (`self.RangedActionParameters`))))
  (set `self.FireProjectileTimerHandle` _returnvalue))

(event `FireProjectile`
  (`/Game/AI/BP_AI_Character.FireProjectile` (`self.OwnerCharacter`))
  (`self.OnNextFire`))

(event `self.OnActionStopped`
  (params (bInActionAborted :type Boolean))
  (bind _owneractor (`self.OwnerActor`))
  (`KismetSystemLibrary.K2_ClearAndInvalidateTimerHandle` _owneractor (`self.FireProjectileTimerHandle`))
  (`KismetSystemLibrary.K2_ClearAndInvalidateTimerHandle` _owneractor (`self.RangedActionTimerHandle`)))
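; BP_Action_Death is the gameplay action that runs death for an AI character.
; On init it caches the owning BP_AI_Character and its BP_AI_Controller.
; On start it disables every other owned action through the gameplay action component, stops the controller's behavior tree logic, then calls OnDeath on the character.
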(event `self.OnInitAction`
  (bind _asbp_ai_character (cast `/Game/AI/BP_AI_Character` (`self.OwnerActor`)))
  (bind _output_get (set `self.OwnerCharacter` _asbp_ai_character))
  (bind _asbp_ai_controller (cast `/Game/AI/BP_AI_Controller` (`AIBlueprintHelperLibrary.GetAIController` _output_get)))
  (set `self.OwnerController` _asbp_ai_controller))

(event `self.OnActionStarted`
  (bind _returnvalue (message `GameplayActionOwnerInterface.GetGameplayActionComponent` (`self.OwnerActor`)))
  (bind _returnvalue_2 (message `GameplayActionInterface.GetOwnedActions` _returnvalue))
  (for _array_element _returnvalue_2
    (if (!= _array_element (`self.ActionTag`))
      (bind _returnvalue_3 (message `GameplayActionOwnerInterface.GetGameplayActionComponent` (`self.OwnerActor`)))
      (message `GameplayActionInterface.DisableAction` _returnvalue_3 _array_element)))
  (`BrainComponent.StopLogic` (`/Game/AI/BP_AI_Controller.BehaviorTree` (`self.OwnerController`)) "")
  (`/Game/AI/BP_AI_Character.OnDeath` (`self.OwnerCharacter`)))
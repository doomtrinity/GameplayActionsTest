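; Gameplay action that staggers an AI character for a set duration, spinning it in place.
; On start it saves the pawn mesh's relative transform, then applies the rotation and offset from its StaggerActionParameters.
; Each tick it counts down and yaws the owner at the configured rate, then asks the gameplay action component to stop the action as completed.
; Stopping restores the saved mesh transform.
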(event `self.OnInitAction`
  (bind _asstagger_action_parameters (cast `/Game/Data/Stagger/StaggerActionParameters` (`self.ActionParameters`)))
  (set `self.StaggerActionParameters` _asstagger_action_parameters)
  (bind _asbp_ai_character (cast `/Game/AI/BP_AI_Character` (`self.OwnerActor`)))
  (set `self.OwnerCharacter` _asbp_ai_character))

(event `self.OnActionStarted`
  (bind _staggeractionparameters (`self.StaggerActionParameters`))
  (bind _pawnmesh (`/Game/AI/BP_AI_Character.PawnMesh` (`self.OwnerCharacter`)))
  (set `self.CurrentStaggerTime` (`self.StaggerTimeDuration`))
  (set `self.DefaultMeshLocation` (`SceneComponent.RelativeLocation` _pawnmesh))
  (set `self.DefaultMeshRotation` (`SceneComponent.RelativeRotation` _pawnmesh))
  (`SceneComponent.K2_SetRelativeRotation` _pawnmesh (`/Game/Data/Stagger/StaggerActionParameters.StaggerMeshRotation` _staggeractionparameters) false false)
  (`SceneComponent.K2_SetRelativeLocation` _pawnmesh (`/Game/Data/Stagger/StaggerActionParameters.StaggerMeshOffset` _staggeractionparameters) false false))

(event `self.OnActionStopped`
  (params (bInActionAborted :type Boolean))
  (bind _pawnmesh (`/Game/AI/BP_AI_Character.PawnMesh` (`self.OwnerCharacter`)))
  (`SceneComponent.K2_SetRelativeRotation` _pawnmesh (`self.DefaultMeshRotation`) false false)
  (`SceneComponent.K2_SetRelativeLocation` _pawnmesh (`self.DefaultMeshLocation`) false false))

(event `self.TickAction`
  (params (DeltaTime :type "Float (single-precision)"))
  (bind _output_get (set `self.CurrentStaggerTime` (- (`self.CurrentStaggerTime`) DeltaTime)))
  (if (> _output_get 0.0)
    (`Actor.K2_AddActorWorldRotation` (`self.OwnerActor`) (`KismetMathLibrary.MakeRotator` 0.0 0.0 (* DeltaTime (`/Game/Data/Stagger/StaggerActionParameters.StaggerRotationAnimRate` (`self.StaggerActionParameters`)))) false false)
    (else
      (bind _returnvalue (message `GameplayActionOwnerInterface.GetGameplayActionComponent` (`self.OwnerActor`)))
      (message `GameplayActionInterface.StopAction` _returnvalue (`self.ActionTag`) true))))
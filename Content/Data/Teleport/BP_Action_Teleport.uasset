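; Gameplay action that teleports an AI character to a location near its target, chosen by EQS.
; Tick raises the pawn mesh for a configured duration, then runs EQS_FindTeleportLocation with the target as querier.
; On success it teleports, faces the target and lowers the mesh before completing.
; Query failures deliberately report completion, a failed teleport reports incomplete, and stopping restores the mesh offset if the query is valid.
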(event `self.OnInitAction`
  (bind _asbp_ai_controller (cast `/Game/AI/BP_AI_Controller` (`AIBlueprintHelperLibrary.GetAIController` (`self.OwnerActor`))))
  (set `self.OwnerController` _asbp_ai_controller)
  (bind _asbp_ai_character (cast `/Game/AI/BP_AI_Character` (`self.OwnerActor`)))
  (bind _output_get (set `self.OwnerCharacter` _asbp_ai_character))
  (bind _output_get_2 (set `self.OwnerMesh` (`/Game/AI/BP_AI_Character.PawnMesh` _output_get)))
  (set `self.DefaultMeshLocation` (`SceneComponent.RelativeLocation` _output_get_2))
  (bind _asteleport_action_parameters (cast `/Game/Data/Teleport/TeleportActionParameters` (`self.ActionParameters`)))
  (set `self.AnimDuration` (`/Game/Data/Teleport/TeleportActionParameters.AnimDuration` _asteleport_action_parameters))
  (set `self.AnimSpeed` (`/Game/Data/Teleport/TeleportActionParameters.AnimSpeed` _asteleport_action_parameters)))

(event `self.OnActionStarted`
  (set `self.AnimCurrentTime` 0.0)
  (set `self.bIsTeleportEndAnim` false))

(event `TryTeleport`
  (bind _returnvalue (`EnvQueryManager.RunEQSQuery` (`self.OwnerActor`) "/Game/AI/EQS/EQS_FindTeleportLocation.EQS_FindTeleportLocation" (`/Game/AI/BP_AI_Controller.GetTargetActor` (`self.OwnerController`)) "SingleResult"))
  (bind _output_get (set `self.CachedEQSQuery` _returnvalue))
  (`/Engine/EditorBlueprintResources/StandardMacros.IsValid` _output_get
    (:`Is Valid`
      (add `EnvQueryInstanceBlueprintWrapper.OnQueryFinishedEvent` (`self.CachedEQSQuery`) (delegate `OnQueryFinished`)))
    (:`Is Not Valid`
      (bind _returnvalue_2 (message `GameplayActionOwnerInterface.GetGameplayActionComponent` (`self.OwnerActor`) :!label _label))
      (message `GameplayActionInterface.StopAction` _returnvalue_2 (`self.ActionTag`) true) ; always succeed on purpose
    )))

(event `OnQueryFinished`
  (params (QueryInstance :type "EnvQueryInstanceBlueprintWrapper Object Reference") (QueryStatus :type "EEnvQueryStatus Enum" :default "Processing"))
  (bind _cachedeqsquery (`self.CachedEQSQuery`))
  (switch `EEnvQueryStatus` QueryStatus
    (:`Success`
      (`/Engine/EditorBlueprintResources/StandardMacros.IsValid` _cachedeqsquery
        (:`Is Valid`
          (bind (_resultlocations _returnvalue) (`EnvQueryInstanceBlueprintWrapper.GetQueryResultsAsLocations` _cachedeqsquery))
          (if _returnvalue
            (bind _returnvalue_2 (`Actor.K2_TeleportTo` :`self` (`self.OwnerActor`) :`DestLocation` (`|GetArrayItem` _resultlocations)))
            (if _returnvalue_2
              (set `self.bIsTeleportEndAnim` true)
              (set `self.AnimCurrentTime` 0.0)
              (`self.RotateToFaceTarget`)
              (else
                (bind _returnvalue_3 (message `GameplayActionOwnerInterface.GetGameplayActionComponent` (`self.OwnerActor`)))
                (message `GameplayActionInterface.StopAction` _returnvalue_3 (`self.ActionTag`) false)))
            (else
              (goto _label))))
        (:`Is Not Valid`
          (goto _label))))
    (:`Failed`
      (goto _label))
    (:`Aborted`
      (goto _label))
    (:`OwnerLost`
      (goto _label))
    (:`MissingParam`
      (goto _label))))

(event `self.OnActionStopped`
  (params (bInActionAborted :type Boolean))
  (bind _cachedeqsquery (`self.CachedEQSQuery`))
  (`/Engine/EditorBlueprintResources/StandardMacros.IsValid` _cachedeqsquery
    (:`Is Valid`
      (remove `EnvQueryInstanceBlueprintWrapper.OnQueryFinishedEvent` _cachedeqsquery (delegate `OnQueryFinished`))
      (`SceneComponent.K2_SetRelativeLocation` (`self.OwnerMesh`) (`self.DefaultMeshLocation`) false false))))

(event `self.TickAction`
  (params (DeltaTime :type "Float (single-precision)"))
  (bind _ownermesh (`self.OwnerMesh`))
  (bind _returnvalue (* (`self.CachedDeltaTime`) (`self.AnimSpeed`)))
  (set `self.CachedDeltaTime` DeltaTime)
  (if (> (`self.AnimCurrentTime`) (`self.AnimDuration`))
    (if (`self.bIsTeleportEndAnim`)
      (bind _returnvalue_2 (message `GameplayActionOwnerInterface.GetGameplayActionComponent` (`self.OwnerActor`)))
      (message `GameplayActionInterface.StopAction` _returnvalue_2 (`self.ActionTag`) true)
      (else
        (`self.TryTeleport`)))
    (else
      (set `self.AnimCurrentTime` (+ (`self.AnimCurrentTime`) (`self.CachedDeltaTime`)))
      (`SceneComponent.K2_SetRelativeLocation` _ownermesh (+ (`SceneComponent.RelativeLocation` _ownermesh) (`KismetMathLibrary.MakeVector` 0.0 0.0 (`KismetMathLibrary.SelectFloat` (* _returnvalue -1.0) _returnvalue (`self.bIsTeleportEndAnim`)))) false false))))

(event `RotateToFaceTarget`
  (`Actor.K2_SetActorRotation` (`self.OwnerActor`) (`KismetMathLibrary.MakeRotFromX` (`KismetMathLibrary.Vector_Normal2D` (- (`Actor.K2_GetActorLocation` (`/Game/AI/BP_AI_Controller.GetTargetActor` (`self.OwnerController`))) (`Actor.K2_GetActorLocation` (`self.OwnerActor`))))) false))